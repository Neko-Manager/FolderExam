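; Fire VFX Blueprint that makes a point light flicker like a flame.
; On BeginPlay it plays a timeline, using its Update output as a tick to lerp the light's intensity toward a target.
; The same update triggers a short random Delay that then picks a new random target, giving irregular but slightly smoothed jumps in brightness.
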(event EventBeginPlay
  (Timeline|FlickeringTimeline Play
    (:Update
      (Utilities|FlowControl|Sequence
        (:then_0
          (Rendering|Components|Light|SetIntensity (Variables|Default|GetPointLight_Fire) (Math|Float|Lerp (Variables|/Script/Engine.LightComponentBase|GetIntensity (Variables|Default|GetPointLight_Fire)) (Variables|Default|GetTargetIntensity) 0.6)))
        (:then_1
          (Utilities|FlowControl|Delay (Math|Random|RandomFloatinRange 0.05 0.1))
          (Variables|Default|SetTargetIntensity (Math|Random|RandomFloatinRange 1e+03 1.5e+04)))))))

(fn ConstructionScript)